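; BP_PlayerBullet is the player's projectile, dealing damage to whatever actor its static mesh hits.
; On hit it applies BaseDamage, crediting player controller 0 as instigator and the player character as causer.
; It then stops mesh physics and collision, hides the mesh, deactivates the trail particle and destroys itself after a short delay.
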(event OnComponentHit(StaticMesh)
  (params (HitComponent :type Primitive%20Component%20Object%20Reference) (OtherActor :type Actor%20Object%20Reference) (OtherComp :type Primitive%20Component%20Object%20Reference) (NormalImpulse :type Vector :default "0, 0, 0") (Hit :type Hit%20Result%20Structure%20%28by%20ref%29))
  (bind _staticmesh (Variables|Default|GetStaticMesh))
  (Game|Damage|ApplyDamage OtherActor (Variables|Default|GetBaseDamage) (Game|GetPlayerController 0) (Game|GetPlayerCharacter 0))
  (Physics|SetSimulatePhysics _staticmesh false)
  (Collision|SetCollisionEnabled _staticmesh "NoCollision")
  (Development|SetHiddeninGame _staticmesh true false)
  (Components|Activation|Deactivate (Variables|Default|GetTrailParticle))
  (Utilities|FlowControl|Delay 4.0)
  (Actor|DestroyActor))

(event EventBeginPlay
  (|CallParentFunction) ; This node is disabled and will not be called.\nDrag off pins to build functionality.
)

(event Collision|EventActorBeginOverlap
  (params (OtherActor :type Actor%20Object%20Reference))
  (|CallParentFunction OtherActor) ; This node is disabled and will not be called.\nDrag off pins to build functionality.
)

(event EventTick
  (params (DeltaSeconds :type Float%20%28single-precision%29))
  (|CallParentFunction DeltaSeconds) ; This node is disabled and will not be called.\nDrag off pins to build functionality.
)

(fn ConstructionScript
  (|CallParentFunction))