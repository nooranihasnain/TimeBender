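; Base enemy Blueprint that plays physically animated and shatters on the first damage caused by the player.
; On BeginPlay, SetPhysicalAnim applies physical animation and blended physics simulation to Spine1 and the bodies below it.
; AnyDamage ignores non-player causers, then disables capsule collision, stops movement and hides the skeletal mesh.
; A destructible component spawned in its place breaks with a randomized impulse before the actor is destroyed after a short delay.
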(event EventBeginPlay
  (CallFunction|SetPhysicalAnim true 1e+03 7e+02 1e+03 7e+02))

(event Collision|EventActorBeginOverlap
  (params (OtherActor :type Actor%20Object%20Reference)))

(event EventTick
  (params (DeltaSeconds :type Float%20%28single-precision%29)))

(event Game|Damage|EventAnyDamage
  (params (Damage :type Float%20%28single-precision%29) (DamageType :type Damage%20Type%20Object%20Reference) (InstigatedBy :type Controller%20Object%20Reference) (DamageCauser :type Actor%20Object%20Reference))
  (bind _mesh (Variables|Character|GetMesh))
  (Utilities|Casting|CastToBP_Player DamageCauser)
  (if (not (Variables|Default|GetIsDead))
    (Variables|Default|SetIsDead true)
    (Collision|SetCollisionEnabled (Variables|Collision|GetCapsuleComponent) "NoCollision")
    (Components|Movement|StopMovementImmediately (Variables|Character|GetCharacterMovement))
    (Rendering|SetVisibility _mesh false false)
    (bind _returnvalue (AddComponent|AddDestructibleComponent false (Transformation|GetRelativeTransform _mesh)))
    (Class|DestructibleComponent|SetDestructibleMesh _returnvalue "/Game/Meshes/EnemyModel/EnemyModelNoRig_DM.EnemyModelNoRig_DM")
    (Physics|SetSimulatePhysics _returnvalue true)
    (Class|DestructibleComponent|ApplyDamage _returnvalue 5e+01 (Transformation|GetWorldLocation (Variables|Character|GetMesh)) (Math|Vector|MakeVector (Math|Float|SelectFloat 0.0 1.0 (Math|Random|RandomBool)) (Math|Float|SelectFloat 0.0 1.0 (Math|Random|RandomBool)) (Math|Float|SelectFloat 0.0 1.0 (Math|Random|RandomBool))) 5e+02)
    (Utilities|FlowControl|Delay 1.0)
    (Actor|DestroyActor)))

(fn ConstructionScript)

(fn SetPhysicalAnim
  (params (Is%20Local%20Simulation :type Boolean) (Orientation%20Strength :type Float%20%28single-precision%29) (Angular%20Velocity%20Strength :type Float%20%28single-precision%29) (Position%20Strength :type Float%20%28single-precision%29) (Velocity%20Strength :type Float%20%28single-precision%29))
  (bind _returnvalue (Utilities|Name|MakeLiteralName "Spine1"))
  (bind _physicalanimation (Variables|Default|GetPhysicalAnimation))
  (bind _mesh (Variables|Character|GetMesh))
  (Class|PhysicalAnimationComponent|SetSkeletalMeshComponent _physicalanimation _mesh)
  (Class|PhysicalAnimationComponent|ApplyPhysicalAnimationSettingsBelow _physicalanimation "Spine1" (Utilities|Struct|MakePhysicalAnimationData Is%20Local%20Simulation Orientation%20Strength Angular%20Velocity%20Strength Position%20Strength Velocity%20Strength) true)
  (Class|SkeletalMeshComponent|SetAllBodiesBelowSimulatePhysics _mesh _returnvalue true true)
  (Class|SkeletalMeshComponent|SetAllBodiesBelowPhysicsBlendWeight _mesh _returnvalue (Variables|Default|GetBlend) false true))