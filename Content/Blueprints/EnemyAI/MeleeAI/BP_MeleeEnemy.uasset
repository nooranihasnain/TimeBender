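; BP_MeleeEnemy is a melee enemy character that damages the player through overlaps on a static mesh attached to its MeleeSocket.
; A DidHit flag gates the attack and is never reset here.
; Any damage caused by the player kills it: the attached mesh drops with physics, and a destructible mesh replaces the hidden body and shatters before the actor is destroyed.
; BeginPlay also sets partial physics blend weight below Spine1.
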(event OnComponentBeginOverlap(StaticMesh)
  (params (OverlappedComponent :type Primitive%20Component%20Object%20Reference) (OtherActor :type Actor%20Object%20Reference) (OtherComp :type Primitive%20Component%20Object%20Reference) (OtherBodyIndex :type Integer) (bFromSweep :type Boolean) (SweepResult :type Hit%20Result%20Structure%20%28by%20ref%29))
  ;[1 1 1] Attack
  (bind _asbp_player (Utilities|Casting|CastToBP_Player OtherActor))
  (if (not (Variables|Default|GetDidHit))
    (Game|Damage|ApplyDamage _asbp_player 1.0 (Pawn|GetController) self)
    (Variables|Default|SetDidHit true)))

(event EventBeginPlay
  (|CallParentFunction)
  (Class|SkeletalMeshComponent|SetAllBodiesBelowPhysicsBlendWeight (Variables|Character|GetMesh) (Utilities|Name|MakeLiteralName "Spine1") 0.5 false true))

(event Collision|EventActorBeginOverlap
  (params (OtherActor :type Actor%20Object%20Reference))
  (|CallParentFunction OtherActor) ; This node is disabled and will not be called.\nDrag off pins to build functionality.
)

(event EventTick
  (params (DeltaSeconds :type Float%20%28single-precision%29))
  (|CallParentFunction DeltaSeconds) ; This node is disabled and will not be called.\nDrag off pins to build functionality.
)

(event Game|Damage|EventAnyDamage
  (params (Damage :type Float%20%28single-precision%29) (DamageType :type Damage%20Type%20Object%20Reference) (InstigatedBy :type Controller%20Object%20Reference) (DamageCauser :type Actor%20Object%20Reference))
  (bind _mesh (Variables|Character|GetMesh))
  (bind _staticmesh (Variables|Default|GetStaticMesh))
  ;[1 1 1] Damage System
  (Utilities|Casting|CastToBP_Player DamageCauser)
  (if (not (Variables|Default|GetIsDead))
    (Variables|Default|SetIsDead true)
    (Components|Movement|StopMovementImmediately (Variables|Character|GetCharacterMovement))
    (Transformation|DetachFromComponent _staticmesh "KeepWorld" "KeepWorld" "KeepWorld" true)
    (Collision|SetCollisionEnabled _staticmesh "QueryAndPhysics")
    (Physics|SetSimulatePhysics _staticmesh true)
    (Rendering|SetVisibility _mesh false false)
    (bind _returnvalue (AddComponent|AddDestructibleComponent false (Transformation|GetRelativeTransform _mesh)))
    (Class|DestructibleComponent|SetDestructibleMesh _returnvalue "/Game/Meshes/EnemyModel/EnemyModelNoRig_DM.EnemyModelNoRig_DM")
    (Physics|SetSimulatePhysics _returnvalue true)
    (Class|DestructibleComponent|ApplyDamage _returnvalue 5e+01 (Transformation|GetWorldLocation (Variables|Character|GetMesh)) (Math|Vector|MakeVector 0.0 0.0 1.0) 5e+02)
    (Utilities|FlowControl|Delay 1.0)
    (Actor|DestroyActor)))

(fn ConstructionScript
  (|CallParentFunction)
  (Transformation|AttachComponentToComponent (Variables|Default|GetStaticMesh) (Variables|Character|GetMesh) "MeleeSocket" "KeepRelative" "KeepRelative" "KeepRelative" true))