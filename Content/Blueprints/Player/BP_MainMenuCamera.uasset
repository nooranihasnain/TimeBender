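; Main menu camera actor that shows the title header and drifts between preset menu viewpoints.
; On BeginPlay it creates the W_TitleHeader widget for the first player controller, adds it to the viewport and gives it keyboard focus.
; While IsInMenu is set, each tick lerps the actor toward the ModeTransforms entry at CurrentPosition, using delta time as alpha for an eased, swept move.
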(event EventBeginPlay
  (bind _returnvalue (UserInterface|CreateWidget "/Game/Blueprints/Widgets/MainMenu/W_TitleHeader.W_TitleHeader_C" (Game|GetPlayerController 0)))
  (UserInterface|Viewport|AddtoViewport _returnvalue 0)
  (Widget|SetKeyboardFocus _returnvalue))

(event Collision|EventActorBeginOverlap
  (params (OtherActor :type Actor%20Object%20Reference)))

(event EventTick
  (params (DeltaSeconds :type Float%20%28single-precision%29))
  (if (Variables|Default|GetIsInMenu)
    (Transformation|SetActorTransform (Math|Transform|Lerp(Transform) (Transformation|GetActorTransform) (Utilities|Array|Get(acopy) (Variables|Default|GetModeTransforms) (Variables|Default|GetCurrentPosition)) DeltaSeconds) true)))

(fn ConstructionScript)